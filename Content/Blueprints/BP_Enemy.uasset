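; BP_Enemy is an enemy that chases the TPS player and switches to attacking once it is close enough.
; A three-state machine (Idle, Move, Attack) starts in Idle and runs on Tick.
; Idle caches the player pawn as the target, and Move steers straight at it with movement input until within the stopping distance.
; Attack is a placeholder that only prints a message each tick, with no transition out.
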(event `self.ReceiveBeginPlay`
  (set `self.myState` "NewEnumerator0"))

(event `self.ReceiveTick`
  (params (DeltaSeconds :type "Float (single-precision)"))
  (switch `/Game/Blueprints/EEnemyStateBP` (`self.myState`)
    (:`NewEnumerator0`
      ;[1 1 1] IDLE : 플레이어를 찾고싶다.
      (bind _asbp_tpsplayer (cast `/Game/Blueprints/BP_TPSPlayer` (`GameplayStatics.GetPlayerPawn` 0)))
      (set `self.myTarget` _asbp_tpsplayer)
      (set `self.myState` "NewEnumerator1"))
    (:`NewEnumerator1`
      ;[1 1 1] Move : myTarget을 향해 이동하고싶다.
      (`self.AddMovementInput` (`KismetMathLibrary.Normal` (- (`self.K2_GetActorLocation` (`self.myTarget`)) (`self.K2_GetActorLocation`))))
      (if (> (`self.myStoppingDistance`) (`KismetMathLibrary.Vector_Distance` (`self.K2_GetActorLocation` (`self.myTarget`)) (`self.K2_GetActorLocation`)))
        (set `self.myState` "NewEnumerator2")))
    (:`NewEnumerator2`
      (`KismetSystemLibrary.PrintString` "Attack!"))))

(fn `UserConstructionScript`)